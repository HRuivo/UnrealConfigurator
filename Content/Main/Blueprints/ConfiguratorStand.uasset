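; Configurable stepped display stand that builds its layout at BeginPlay and opens a configuration widget targeting itself.
; InitializeStand rebuilds instanced mesh steps from StepCount and Width, spacing them by mesh bounds and attaching a slot actor atop each exposed step piece.
; Slots are indexed in StandSlotMap and bind selection events, while NotifySlotSelected rebroadcasts selection.
; LoadPreset resizes and fills slots from a data table; SavePreset is empty and LoadSavedPresets discards its rows.
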(event Custom|DEBUG%20Load%20Preset
  (CallFunction|LoadPreset (Variables|Default|GetDebug%20Preset%20Name)))

(event EventBeginPlay
  (CallFunction|InitializeStand)
  (bind _returnvalue (UserInterface|CreateWidget "/Game/Main/UI/ConfigurationWidget.ConfigurationWidget_C" 0 self))
  (UserInterface|Viewport|AddtoViewport _returnvalue 0))

(fn ConstructionScript)

(fn AddStep
  (params (Level :type Integer))
  (bind _self self)
  (bind _pieces (Variables|Default|GetPieces))
  (bind _step_count (Variables|Default|GetStep%20Count))
  (bind _step_count_2 (Variables|Default|GetStep%20Count))
  (bind _width (Variables|Default|GetWidth))
  (bind _returnvalue (- _width 1))
  (bind _returnvalue_2 (Math|Integer|Min(Integer) _step_count_2 Level))
  (bind _staticmesh (Variables|/Script/Engine.StaticMeshComponent|GetStaticMesh _pieces))
  (bind _returnvalue_3 (StaticMesh|GetBounds _staticmesh))
  (bind _returnvalue_4 (- _step_count _returnvalue_2))
  (bind _returnvalue_5 (* (.boxextent _returnvalue_3) 2.0))
  (bind (_x _y _z) (Math|Vector|BreakVector _returnvalue_5))
  (for _index (range 0 _returnvalue)
    (for _index_2 (range 0 _returnvalue_4)
      (Components|InstancedStaticMesh|AddInstance (Variables|Default|GetPieces) (Math|Transform|MakeTransform (Math|Vector|MakeVector (* _index_2 _x) (- (* _index _y) (* (/ _returnvalue 2) _y)) (* _returnvalue_2 _z))))
      (if (== _index_2 _returnvalue_4)
        (bind _returnvalue_6 (Game|SpawnActorfromClass (Variables|Default|GetSlot%20Type) (Math|Transform|MakeTransform (+ (Math|Vector|MakeVector (* _index_2 _x) (- (* _index _y) (* (/ _returnvalue 2) _y)) (* _returnvalue_2 _z)) "0, 0,55.000000")) "AlwaysSpawn" 0 _self 0))
        (EventDispatchers|BindEventtoOnSelected _returnvalue_6 (EventDispatchers|CreateEvent :!event NotifySlotSelected))
        (Transformation|AttachActorToActor _returnvalue_6 _self "None" "KeepWorld" "KeepWorld" "KeepWorld" false)
        (Utilities|Map|Add (Variables|Default|GetStand%20Slot%20Map) (Utilities|Map|Length (Variables|Default|GetStand%20Slot%20Map)) _returnvalue_6)
        (Transformation|SetActorRelativeTransform _returnvalue_6 (Math|Transform|MakeTransform (+ (Math|Vector|MakeVector (* _index_2 _x) (- (* _index _y) (* (/ _returnvalue 2) _y)) (* _returnvalue_2 _z)) "0, 0,55.000000")) false false)))))

(fn InitializeStand
  (Components|InstancedStaticMesh|ClearInstances (Variables|Default|GetPieces))
  (bind _values (Utilities|Map|Values (Variables|Default|GetStand%20Slot%20Map)))
  (for _array_element _values
    (Actor|DestroyActor _array_element))
  (Utilities|Map|Clear (Variables|Default|GetStand%20Slot%20Map))
  (for _index (range 1 (Variables|Default|GetStep%20Count))
    (CallFunction|AddStep _index)))

(fn NotifySlotSelected
  (params (Selected%20Slot :type Stand%20Slot%20Standart%20Object%20Reference))
  (Default|CallOnNewSlotSelected Selected%20Slot))

(fn SavePreset)

(fn LoadPreset
  (params (Preset%20Name :type Name))
  (bind _returnvalue (Utilities|GetDataTableRow (Variables|Default|GetPreset%20DataTable) Preset%20Name)
    (:then
      (Variables|Default|SetStep%20Count (.StepCount (Utilities|Struct|BreakPresetData _returnvalue)))
      (Variables|Default|SetWidth (.StandWidth (Utilities|Struct|BreakPresetData _returnvalue)))
      (CallFunction|InitializeStand)
      (for _array_element (.ObjectData (Utilities|Struct|BreakPresetData _returnvalue))
        (Default|AddObject (.Value (Utilities|Map|Find (Variables|Default|GetStand%20Slot%20Map) (.SlotIndex (Utilities|Struct|BreakPresetObjectData _array_element)))) (.ObjectClass (Utilities|Struct|BreakPresetObjectData _array_element)) (.Material (Utilities|Struct|BreakPresetObjectData _array_element)) (.Visible (Utilities|Struct|BreakPresetObjectData _array_element)))))))

(fn LoadSavedPresets
  (bind _preset_datatable (Variables|Default|GetPreset%20DataTable))
  (bind _outrownames (DataTable|GetDataTableRowNames _preset_datatable))
  (for _array_element _outrownames
    (bind _returnvalue (Utilities|GetDataTableRow _preset_datatable _array_element))))