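; ConfiguratorGameMode is the game mode for a configurator scene, setting up the stand and the main UI when play begins.
; On BeginPlay it stores the first ConfiguratorStand found in the level as MainConfiguratorStand, spawning one if none exists or the found one is invalid.
; It then creates the MainWidget and adds it to the viewport.
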(event EventBeginPlay
  (bind _outactors (Actor|GetAllActorsOfClass "/Game/Main/Blueprints/ConfiguratorStand.ConfiguratorStand_C"))
  (if (> (Utilities|Array|Length _outactors) 0)
    (Utilities|IsValid (Utilities|Array|Get(acopy) _outactors)
      (:Is%20Valid
        (Variables|Default|SetMain%20Configurator%20Stand (Utilities|Array|Get(acopy) _outactors)))
      (:Is%20Not%20Valid
        (bind _returnvalue (Game|SpawnActorfromClass "/Game/Main/Blueprints/ConfiguratorStand.ConfiguratorStand_C" (Math|Transform|MakeTransform "0, 0, 0" "0, 0, 0" "1,1,1") "AlwaysSpawn" 0 0 :!label _label))
        (Variables|Default|SetMain%20Configurator%20Stand _returnvalue)))
    (else
      (goto _label)))
  (bind _returnvalue_2 (UserInterface|CreateWidget "/Game/Main/UI/MainWidget.MainWidget_C"))
  (UserInterface|Viewport|AddtoViewport _returnvalue_2 0))

(fn ConstructionScript)