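; StandSlot_Standart is a selectable slot actor that holds one spawned object at its SpawnSocket.
; Its Plane shows on cursor hover, and clicking it fires an OnSelected dispatcher with the slot itself.
; AddObject spawns the given class and replaces any current object, while other functions remove it, toggle its visibility or report its state.
; Destroying the slot also destroys the object it holds.
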(event OnClicked(Plane)
  (params (TouchedComponent :type Primitive%20Component%20Object%20Reference) (ButtonPressed :type Key%20Structure))
  (Default|CallOnSelected self))

(event OnBeginCursorOver(Plane)
  (params (TouchedComponent :type Primitive%20Component%20Object%20Reference))
  (Development|SetHiddeninGame (Variables|Default|GetPlane) false false))

(event OnEndCursorOver(Plane)
  (params (TouchedComponent :type Primitive%20Component%20Object%20Reference))
  (Development|SetHiddeninGame (Variables|Default|GetPlane) true false))

(event Custom|OnDestroyed_Event_0
  (params (DestroyedActor :type Actor%20Object%20Reference))
  (Utilities|IsValid (Variables|Default|GetCurrent%20Object)
    (:Is%20Valid
      (CallFunction|RemoveCurrentObject))))

(event EventBeginPlay
  (EventDispatchers|AssignOnDestroyed (delegate Custom|OnDestroyed_Event_0)))

(event EventDestroyed
  (CallFunction|RemoveCurrentObject))

(fn ConstructionScript)

(fn AddObject
  (params (New%20Object%20Class :type Configurable%20Object%20Class%20Reference))
  (bind _returnvalue (Game|SpawnActorfromClass New%20Object%20Class (Transformation|GetWorldTransform (Variables|Default|GetSpawn%20Socket)) "AlwaysSpawn" self 0))
  (Utilities|IsValid (Variables|Default|GetCurrent%20Object)
    (:Is%20Valid
      (CallFunction|RemoveCurrentObject))
    (:Is%20Not%20Valid
      _))
  (Variables|Default|SetCurrent%20Object _returnvalue))

(fn RemoveCurrentObject
  (Utilities|IsValid (Variables|Default|GetCurrent%20Object)
    (:Is%20Valid
      (Actor|DestroyActor (Variables|Default|GetCurrent%20Object))
      (Variables|Default|SetCurrent%20Object 0))))

(fn SetObjectVisibility
  (params (Visible :type Boolean))
  (if (CallFunction|HasObjectAssigned)
    (Class|VisibilityToggler|SetVisibility(Message) (Variables|Default|GetCurrent%20Object) Visible)))

(fn HasObjectAssigned
  (return (Utilities|IsValid (Variables|Default|GetCurrent%20Object))))

(fn IsCurrentObjectVisible
  (if (CallFunction|HasObjectAssigned)
    (return (not (Variables|/Script/Engine.Actor|GetbHidden (Variables|Default|GetCurrent%20Object))))
    (else
      (return false))))