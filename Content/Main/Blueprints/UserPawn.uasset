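; UserPawn is the player pawn for viewing configurator objects, switching between free-fly movement and a focus view on a selected object.
; Free mode moves along control-rotation axes, while focus mode blocks movement and lets zoom inputs change the spring arm length.
; FocusObject moves the pawn to the object's focus location, or slightly above a non-configurator actor, and activates FocusCamera.
; ClearFocus restores the main camera at FocusCamera's position.
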(event Input|ActionEvents|InputActionZoomIn
  (params (Key :type Key%20Structure))
  (bind _springarm (Variables|Default|GetSpringArm))
  (:Pressed
    (if (Variables|Default|GetIn%20Focus%20Mode)
      (Variables|/Script/Engine.SpringArmComponent|SetTargetArmLength _springarm (- (Variables|/Script/Engine.SpringArmComponent|GetTargetArmLength _springarm) (Variables|Default|GetZoom%20Strength))))))

(event Input|ActionEvents|InputActionZoomOut
  (params (Key :type Key%20Structure))
  (bind _springarm (Variables|Default|GetSpringArm))
  (:Pressed
    (if (Variables|Default|GetIn%20Focus%20Mode)
      (Variables|/Script/Engine.SpringArmComponent|SetTargetArmLength _springarm (+ (Variables|/Script/Engine.SpringArmComponent|GetTargetArmLength _springarm) (Variables|Default|GetZoom%20Strength))))))

(event Input|AxisEvents|InputAxisCameraYaw
  (params (AxisValue :type Float%20%28single-precision%29))
  (Pawn|Input|AddControllerYawInput AxisValue))

(event Input|AxisEvents|InputAxisCameraPitch
  (params (AxisValue :type Float%20%28single-precision%29))
  (Pawn|Input|AddControllerPitchInput AxisValue))

(event Input|AxisEvents|InputAxisMoveForward
  (params (AxisValue :type Float%20%28single-precision%29))
  (if (not (Variables|Default|GetIn%20Focus%20Mode))
    (Pawn|Input|AddMovementInput (Math|Vector|GetForwardVector (Pawn|GetControlRotation :!class /Script/Engine.Pawn)) AxisValue false)))

(event Input|AxisEvents|InputAxisMoveRight
  (params (AxisValue :type Float%20%28single-precision%29))
  (if (not (Variables|Default|GetIn%20Focus%20Mode))
    (Pawn|Input|AddMovementInput (Math|Vector|GetRightVector (Pawn|GetControlRotation :!class /Script/Engine.Pawn)) AxisValue false)))

(event Input|AxisEvents|InputAxisMoveUpward
  (params (AxisValue :type Float%20%28single-precision%29))
  (if (not (Variables|Default|GetIn%20Focus%20Mode))
    (Pawn|Input|AddMovementInput (Math|Vector|GetUpVector (Pawn|GetControlRotation :!class /Script/Engine.Pawn)) AxisValue false)))

(fn ConstructionScript)

(fn FocusObject
  (params (Object%20to%20Focus :type Actor%20Object%20Reference))
  (Variables|Default|SetCurrent%20Target%20Object Object%20to%20Focus)
  (Variables|Default|SetIn%20Focus%20Mode true)
  (Transformation|SetActorLocation (select (.bSuccess (Utilities|Casting|CastToBaseConfiguratorObject (Variables|Default|GetCurrent%20Target%20Object))) (Class|BaseConfiguratorObject|GetFocusLocation (.AsBase%20Configurator%20Object (Utilities|Casting|CastToBaseConfiguratorObject (Variables|Default|GetCurrent%20Target%20Object)))) (+ (Transformation|GetActorLocation (Variables|Default|GetCurrent%20Target%20Object)) "0, 0,15.000000")) false false)
  (Components|Activation|SetActive (Variables|Default|GetCamera) false false)
  (Components|Activation|SetActive (Variables|Default|GetFocus%20Camera) true false))

(fn ClearFocus
  (Variables|Default|SetIn%20Focus%20Mode false)
  (Variables|Default|SetCurrent%20Target%20Object 0)
  (Components|Activation|Deactivate (Variables|Default|GetFocus%20Camera))
  (Components|Activation|Activate (Variables|Default|GetCamera) false)
  (Transformation|SetActorLocation (Transformation|GetWorldLocation (Variables|Default|GetFocus%20Camera)) false false))

(fn IsinFocusMode
  (return (Variables|Default|GetIn%20Focus%20Mode)))