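; BP_BaseConfigObject is a base Blueprint actor for configurable objects, exposing control over visibility and the material on its mesh.
; On BeginPlay it caches the mesh's slot 0 material as the original.
; Events show or hide the whole actor, apply a new material to slot 0, or restore the cached one.
; Query functions report current visibility and the assigned material.
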(event EventBeginPlay
  (Variables|Default|SetOriginal%20Material (Rendering|Material|GetMaterial (Variables|Default|GetMesh) 0)))

(event EventSetVisibility
  (params (IsVisible :type Boolean))
  (Rendering|SetActorHiddenInGame (not IsVisible)))

(event EventSetMaterial
  (params (NewMaterial :type Material%20Interface%20Object%20Reference))
  (Rendering|Material|SetMaterial (Variables|Default|GetMesh) 0 NewMaterial))

(event EventResetMaterial
  (Rendering|Material|SetMaterial (Variables|Default|GetMesh) 0 (Variables|Default|GetOriginal%20Material)))

(fn ConstructionScript)

(fn IsVisible
  (return (not (Variables|Default|GetbHidden))))

(fn GetAssignedMaterial
  (return (Rendering|Material|GetMaterial (Variables|Default|GetMesh) 0)))