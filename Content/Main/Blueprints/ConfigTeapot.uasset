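; ConfigTeapot is a teapot actor whose visibility and material can be changed through custom events.
; Visibility events show, hide or toggle the whole actor via its hidden-in-game state.
; The construction script caches the mesh's slot 0 material, so ResetMaterial can restore it after SetMaterial swaps in another.
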(event EventSetVisibility
  (params (Visible :type Boolean))
  (Rendering|SetActorHiddenInGame (not Visible)))

(event EventToggleVisibility
  (CallFunction|SetVisibility (Variables|Default|GetbHidden)))

(event EventResetMaterial
  (Rendering|Material|SetMaterial (Variables|Default|GetMesh) 0 (Variables|Default|GetOriginal%20Material)))

(event EventSetMaterial
  (params (New%20Material :type Material%20Interface%20Object%20Reference))
  (Rendering|Material|SetMaterial (Variables|Default|GetMesh) 0 New%20Material))

(fn ConstructionScript
  (Variables|Default|SetOriginal%20Material (Rendering|Material|GetMaterial (Variables|Default|GetMesh) 0)))